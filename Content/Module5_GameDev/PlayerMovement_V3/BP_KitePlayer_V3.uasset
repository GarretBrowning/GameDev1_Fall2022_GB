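; Player Blueprint with hand-written movement: horizontal axis input along X, custom gravity and a hold-to-charge jump, all through SetActorLocation.
; Tick builds a capped hold time while Jump is held on the ground, otherwise applies gravity with a swept move whose blocking hit sets IsGrounded.
; Releasing Jump while grounded applies one displacement scaled by hold time and frame delta.
; Disconnected IsJumping logic remains in the graph.
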(event `CalculateJumpHoldTime`
  ;[0 0.3 0] Calculate Jump Hold Time
  (bind _output_get (set `self.JumpHoldTime` (`KismetMathLibrary.FMin` (+ (`self.JumpHoldTime`) (`self.DeltaTime`)) (`self.MaxJumpHoldTime`))))
  (`KismetSystemLibrary.PrintString` (`KismetStringLibrary.Concat_StrStr` "Jump Hold Time: " (`KismetStringLibrary.Conv_DoubleToString` _output_get))))

(event `InputAxis|MoveHorizontal`
  (params (AxisValue :type "Float (single-precision)"))
  ;[0 0.3 0] Horizontal Movement (X-Axis)
  (`self.K2_SetActorLocation` (+ (`KismetMathLibrary.MakeVector` (* (* AxisValue (`self.DeltaTime`)) (`self.MovementSpeed`))) (`self.K2_GetActorLocation`))))

(event `self.ReceiveTick`
  (params (DeltaSeconds :type "Float (single-precision)"))
  ;[0 0.3 0] Add JumpForce Each Frame We Are Jumping.
  (set `self.DeltaTime` DeltaSeconds)
  (if (and (`self.bJumpButtonHeld`) (`self.bIsGrounded`))
    (`self.CalculateJumpHoldTime`)
    (else
      (`self.ApplyGravitationalForce`))))

(event `ApplyJumpForce`
  ;[0 0.3 0] Apply Jump Force
  (`self.K2_SetActorLocation` (+ (* (* (`self.JumpForce`) (`self.JumpHoldTime`)) (`self.DeltaTime`)) (`self.K2_GetActorLocation`)) true))

(event `ApplyGravitationalForce`
  ;[0 0.3 0] Apply Gravity. Checks If Grounded.
  (bind _sweephitresult (`self.K2_SetActorLocation` (- (`self.K2_GetActorLocation`) (* (`self.Gravity`) (`self.DeltaTime`))) true))
  (set `self.bIsGrounded` (`GameplayStatics.BreakHitResult` _sweephitresult)))

(event `InputAction|Jump`
  (params (Key :type "Key Structure"))
  ;[0 0.3 0] Set If Jumping Or Not (Only if Grounded).
  (:`Pressed`
    (set `self.bJumpButtonHeld` true))
  (:`Released`
    (set `self.bJumpButtonHeld` false)
    (if (`self.bIsGrounded`)
      (`self.ApplyJumpForce`)
      (set `self.JumpHoldTime` 0.0)
      (else
        (set `self.JumpHoldTime` 0.0)))))

(fn `UserConstructionScript`)