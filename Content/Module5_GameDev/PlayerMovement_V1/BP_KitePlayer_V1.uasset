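; BP_KitePlayer_V1 is a first-version player Blueprint that handles horizontal movement and jumping by directly setting actor location each frame.
; The horizontal axis offsets X without sweeping, scaled by speed and delta time cached on Tick.
; Tick applies jump force while jump is held, otherwise sweeps down by gravity and sets the grounded flag from the blocking hit.
; Jumps start only when grounded.
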(event `InputAxis|MoveHorizontal`
  (params (AxisValue :type "Float (single-precision)"))
  ;[0 0.3 0] Horizontal Movement (X-Axis)
  (`self.K2_SetActorLocation` (+ (`KismetMathLibrary.MakeVector` (* (* AxisValue (`self.DeltaTime`)) (`self.MovementSpeed`))) (`self.K2_GetActorLocation`))))

(event `self.ReceiveTick`
  (params (DeltaSeconds :type "Float (single-precision)"))
  ;[0 0.3 0] Add JumpForce Each Frame We Are Jumping.
  (set `self.DeltaTime` DeltaSeconds)
  (if (`self.bIsJumping`)
    (`self.K2_SetActorLocation` (+ (* (`self.JumpForce`) (`self.DeltaTime`)) (`self.K2_GetActorLocation`)) true)
    (else
      ;[0 0.3 0] If Not Jumping, Add Gravity Each Frame. Sets Is Grounded Upon Blocking Sweep Hit.
      (bind _sweephitresult (`self.K2_SetActorLocation` (- (`self.K2_GetActorLocation`) (* (`self.Gravity`) (`self.DeltaTime`))) true))
      (set `self.bIsGrounded` (`GameplayStatics.BreakHitResult` _sweephitresult)))))

(event `InputAction|Jump`
  (params (Key :type "Key Structure"))
  ;[0 0.3 0] Set If Jumping Or Not (Only if Grounded).
  (:`Pressed`
    (if (`self.bIsGrounded`)
      (set `self.bIsJumping` true)
      (`KismetSystemLibrary.PrintString` (`KismetStringLibrary.Concat_StrStr` "Is Jumping? " (`KismetStringLibrary.Conv_BoolToString` (`self.bIsJumping`))) :!label _label)))
  (:`Released`
    (set `self.bIsJumping` false)
    (goto _label)))

(fn `UserConstructionScript`)