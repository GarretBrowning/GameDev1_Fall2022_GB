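; BP_Kite is a Paper2D Blueprint for the Kite sprite that switches between its flipbook animations on player input.
; On BeginPlay it creates the WBP_UI widget and adds it to the viewport.
; The Idle, Flirt, Run and Powerup input actions each set the matching flipbook on the PaperFlipbook component when pressed, with no state machine or release handling.
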(event `self.ReceiveBeginPlay`
  ;[1 1 1] Create UI Layout to Add to Viewport
  (bind _returnvalue (`|CreateWidget` "/Game/Module4_GameDev/WBP_UI.WBP_UI_C"))
  (`UserWidget.AddToViewport` _returnvalue 0))

(event `InputAction|Idle`
  (params (Key :type "Key Structure"))
  ;[1 1 1] Flipbook Animation Selection
  (:`Pressed`
    (`PaperFlipbookComponent.SetFlipbook` (`self.PaperFlipbook`) "/Game/Art/Flipbooks/Kite_Idle.Kite_Idle")))

(event `InputAction|Flirt`
  (params (Key :type "Key Structure"))
  ;[1 1 1] Flipbook Animation Selection
  (:`Pressed`
    (`PaperFlipbookComponent.SetFlipbook` (`self.PaperFlipbook`) "/Game/Art/Flipbooks/Kite_Flirt.Kite_Flirt")))

(event `InputAction|Run`
  (params (Key :type "Key Structure"))
  ;[1 1 1] Flipbook Animation Selection
  (:`Pressed`
    (`PaperFlipbookComponent.SetFlipbook` (`self.PaperFlipbook`) "/Game/Art/Flipbooks/Kite_Run.Kite_Run")))

(event `InputAction|Powerup`
  (params (Key :type "Key Structure"))
  ;[1 1 1] Flipbook Animation Selection
  (:`Pressed`
    (`PaperFlipbookComponent.SetFlipbook` (`self.PaperFlipbook`) "/Game/Art/Flipbooks/Kite_Powerup.Kite_Powerup")))

(fn `UserConstructionScript`)